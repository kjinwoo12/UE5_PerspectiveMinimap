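; BP_MapIconComponent is a scene component that gives its owner a map icon by managing a separate BP_MapIcon actor.
; On BeginPlay it spawns that actor with its own Material and IconTexture, attaches it to itself with snap-to-target rules and prints whether attachment succeeded.
; On EndPlay it destroys the icon actor if still valid, tying the icon's lifetime to the component; Tick is empty.
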(event EventBeginPlay
  (bind _returnvalue (Components|GetOwner))
  (bind _returnvalue_2 (Game|SpawnActorfromClass "/PerspectiveMinimap/BP_MapIcon.BP_MapIcon_C" (Math|Transform|MakeTransform "0, 0, 0" (Variables|Default|GetRelativeRotation) (Variables|Default|GetRelativeScale3D)) "AlwaysSpawn" "MultiplyWithRoot" _returnvalue (Variables|Params|GetMaterial) (Variables|파라미터|GetIconTexture) (Variables|/Script/Engine.Actor|GetInstigator _returnvalue)))
  (bind _output_get (Variables|Private|SetMapIconActor _returnvalue_2))
  (bind _returnvalue_3 (Transformation|AttachComponentToComponent _output_get self "None" "SnapToTarget" "SnapToTarget" "SnapToTarget" false))
  (if _returnvalue_3
    (Development|PrintString "BP_MapIconComponent::BeginPlay - succeed to attach actor to component")
    (else
      (Development|PrintString "BP_MapIconComponent::BeginPlay - fail to attach actor to component"))))

(event EventTick
  (params (DeltaSeconds :type Float%20%28single-precision%29)))

(event EventEndPlay
  (params (EndPlayReason :type EEndPlayReason%20Enum :default "Destroyed"))
  (bind _mapiconactor (Variables|Private|GetMapIconActor))
  (Utilities|IsValid _mapiconactor
    (:Is%20Valid
      (Actor|DestroyActor _mapiconactor))))